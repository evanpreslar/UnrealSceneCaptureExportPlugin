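; Stereo cubemap capture actor that exports per-face scene renders for a left and right eye as HDR files.
; The construction script groups twelve SceneCapture2D components into two six-direction eye arrays, offset to opposite sides on local Y by half of EyeDistance.
; On BeginPlay it exports each capture's render target to a hardcoded local folder, named by eye and face index.
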(event `self.ReceiveBeginPlay`
  (for (_array_element _array_index) (`self.Left Eyes`)
    (`KismetRenderingLibrary.ExportRenderTarget` (`SceneCaptureComponent2D.TextureTarget` _array_element) "E:\\Files\\Renders" (`KismetStringLibrary.Concat_StrStr` "CubeMapRender_" (`KismetStringLibrary.Concat_StrStr` (`KismetStringLibrary.Concat_StrStr` "Left" (`KismetStringLibrary.Conv_IntToString` _array_index)) ".hdr"))))
  (for (_array_element_2 _array_index_2) (`self.Right Eyes`)
    (`KismetRenderingLibrary.ExportRenderTarget` (`SceneCaptureComponent2D.TextureTarget` _array_element_2) "E:\\Files\\Renders" (`KismetStringLibrary.Concat_StrStr` "CubeMapRender_" (`KismetStringLibrary.Concat_StrStr` (`KismetStringLibrary.Concat_StrStr` "Right" (`KismetStringLibrary.Conv_IntToString` _array_index_2)) ".hdr")))))

(fn `UserConstructionScript`
  (bind _eyedistance (`self.EyeDistance`))
  (bind _output_get (set `self.Left Eyes` (`|MakeArray` (`self.LeftEyeCaptureLeft`) (`self.LeftEyeCaptureRight`) (`self.LeftEyeCaptureUp`) (`self.LeftEyeCaptureDown`) (`self.LeftEyeCaptureBack`) (`self.LeftEyeCaptureForward`))))
  (for _array_element _output_get
    (`SceneComponent.K2_SetRelativeLocation` _array_element (`KismetMathLibrary.MakeVector` 0.0 (/ _eyedistance 2.0)) false false))
  (bind _output_get_2 (set `self.Right Eyes` (`|MakeArray` (`self.RightEyeCaptureLeft`) (`self.RightEyeCaptureRight`) (`self.RightEyeCaptureUp`) (`self.RightEyeCaptureDown`) (`self.RightEyeCaptureBack`) (`self.RightEyeCaptureForward`))))
  (for _array_element_2 _output_get_2
    (`SceneComponent.K2_SetRelativeLocation` _array_element_2 (`KismetMathLibrary.MakeVector` 0.0 (/ _eyedistance -2.0)) false false)))