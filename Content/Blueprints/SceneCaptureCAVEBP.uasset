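; Scene capture Blueprint that renders a frame sequence to files, apparently for CAVE display, then quits the game.
; While IsActive, each Tick skips a configured number of lead-in frames, then calls CaptureAndExport2DCaptureSet until the frame limit is reached.
; Each capture set takes eye distance, longitudinal and latitudinal divisions, resolution and FOV.
; Garbage collection runs at a configurable frame interval, and progress prints only to the log.
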(event `self.ReceiveBeginPlay`)

(event `self.ReceiveTick`
  (params (DeltaSeconds :type "Float (single-precision)"))
  (if (`self.IsActive`) :!pinned true
    (if (>= (`self.Current Frame Num `) (`self.NumFramesToSkip`)) :!pinned true
      (if (> (`self.MaxFramesToCapture`) (- (`self.Current Frame Num `) (`self.NumFramesToSkip`))) :!pinned true
        (`KismetSystemLibrary.PrintString` (`KismetStringLibrary.BuildString_Int` "Rendering Frame " "" (`self.Current Frame Num `)) false true (struct :`G` 1.0 :`B` 0.189364 :`A` 1.0) 0.0)
        (`SceneCaptureCubeHDRRenderBPLibrary.CaptureAndExport2DCaptureSet` (`self.CaptureComponent2D`) (`self.Eye Distance`) (`self.NumLongitudinalDivisions`) (`self.NumLatitudinalDivisions`) (`self.Render Target X Resolution`) (`self.Render Target Y Resolution`) (`self.FOVAngle`) (`self.FilePath`) (`self.BaseFileName`) (`self.Current Frame Num `))
        (`KismetSystemLibrary.PrintString` (`KismetStringLibrary.BuildString_Int` "Rendered Frame " "" (`self.Current Frame Num `)) false true (struct :`G` 1.0 :`B` 0.189364 :`A` 1.0) 0.0)
        (set `self.Current Frame Num ` (+ (`self.Current Frame Num `) 1) :!label _label)
        (if (== (mod (`self.Current Frame Num `) (`self.GarbageCollectAfterNumFrames`)) 0) :!pinned true
          (`KismetSystemLibrary.PrintString` "Scheduling Garbage Collection" false true (struct :`G` 1.0 :`B` 0.189364 :`A` 1.0))
          (`KismetSystemLibrary.CollectGarbage`))
        (elif (== (`self.MaxFramesToCapture`) (- (`self.Current Frame Num `) (`self.NumFramesToSkip`))) :!pinned true
          (`KismetSystemLibrary.PrintString` (`KismetStringLibrary.BuildString_Int` "All Frames Rendered (" "" (`self.MaxFramesToCapture`) " Frames)") false true (struct :`G` 1.0 :`B` 0.189364 :`A` 1.0) 0.0)
          (`KismetSystemLibrary.QuitGame` null "Quit")))
      (else
        (`KismetSystemLibrary.PrintString` (`KismetStringLibrary.BuildString_Int` "Skipping Frame " "" (`self.Current Frame Num `)) false true (struct :`G` 1.0 :`B` 0.189364 :`A` 1.0) 0.0)
        (goto _label)))))

(fn `UserConstructionScript`)